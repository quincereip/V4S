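; Player controller Blueprint, judging by its name, that switches the player between on-foot character and vehicle.
; The ChangePawn event enters when OnEnterBox is set, possessing the vehicle and hiding the character with collision ignored.
; On exit, it restores the character at ExitLocation with the vehicle's rotation and re-possesses it.
; It adds and removes the HUD widget, plus a crosshair for vehicles tagged Armed.
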(event `ChangePawn`
  (bind _charref (`self.CharRef`))
  (bind _entervehicle (`self.EnterVehicle`))
  (bind _charref_2 (`self.CharRef`))
  (bind _returnvalue (`self.ActorHasTag` _entervehicle "Armed"))
  (bind (_returnvalue_location _returnvalue_rotation) (`KismetMathLibrary.BreakTransform` (`SceneComponent.K2_GetComponentToWorld` (`Actor.RootComponent` (`self.EnterVehicle`)))))
  ;[1 1 1] Change Pawn
  (if (`self.InCar`)
    ;[1 1 1] Vehicle Settings
    (`self.SetActorHiddenInGame` _charref_2 false)
    (`PrimitiveComponent.SetCollisionResponseToAllChannels` (`Character.CapsuleComponent` _charref_2) "ECR_Block")
    (`self.K2_SetActorTransform` _charref_2 (`KismetMathLibrary.MakeTransform` (`SceneComponent.K2_GetComponentLocation` (`self.ExitLocation`)) _returnvalue_rotation) false false)
    (`self.Possess` (`Pawn.GetController` (`self.EnterVehicle`)) _charref_2)
    (set `self.InCar` false)
    (`Widget.RemoveFromParent` (stale _returnvalue_2))
    (if _returnvalue
      (`Widget.RemoveFromParent` (stale _returnvalue_3)))
    (else
      ;[1 1 1] 3rd Person Settings
      (if (`self.OnEnterBox`)
        (`self.Possess` (`Pawn.GetController` _charref) _entervehicle)
        (`self.SetActorHiddenInGame` _charref true)
        (`PrimitiveComponent.SetCollisionResponseToAllChannels` (`Character.CapsuleComponent` _charref) "ECR_Ignore")
        (set `self.InCar` true)
        (bind _returnvalue_2 (`|CreateWidget` "/Game/VanVehicle/UI/W_HUD.W_HUD_C"))
        (`UserWidget.AddToViewport` _returnvalue_2 0)
        (if _returnvalue
          (bind _returnvalue_3 (`|CreateWidget` "/Game/VanVehicle/UI/W_Crosshair.W_Crosshair_C"))
          (`UserWidget.AddToViewport` _returnvalue_3 0))))))

(fn `UserConstructionScript`)